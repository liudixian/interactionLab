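; BP_oscFaceData receives face-tracking data over OSC, apparently from MediaPipe, to drive a face mesh.
; One address handler prints the path and builds a transform from six floats, reordering rotation with one axis negated and using a fixed scale.
; The other splits floats into scaled, X-flipped landmark vectors, then calls CreateFace on the Mesh after a short delay.
; The UpdateMesh call is unconnected, and Tick does nothing.
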(event `self.Match_Address_01`
  (params (AddressPattern :type "OSCAddress Structure (by ref)") (Message :type "OSCMessage Structure (by ref)") (IPAddress :type String) (Port :type Integer))
  (bind _returnvalue (`OSCManager.GetOSCAddressFullPath` AddressPattern))
  (`KismetSystemLibrary.PrintString` _returnvalue)
  (bind _values (`OSCManager.GetAllFloats` Message))
  (set `self.Transforms` (`KismetMathLibrary.MakeTransform` (`KismetMathLibrary.MakeVector` (`|GetArrayItem` _values) (`|GetArrayItem` _values 1) (`|GetArrayItem` _values 2)) (`KismetMathLibrary.MakeRotator` (`|GetArrayItem` _values 5) (`|GetArrayItem` _values 4) (* (`|GetArrayItem` _values 3) -1.0)) (0.3 0.3 0.3))))

(event `self.ReceiveTick`
  (params (DeltaSeconds :type "Float (single-precision)")))

(event `self.Match_Address_02`
  (params (AddressPattern :type "OSCAddress Structure (by ref)") (Message :type "OSCMessage Structure (by ref)") (IPAddress :type String) (Port :type Integer))
  (bind _values (`OSCManager.GetAllFloats` Message))
  (bind _vecout (`/GenartLib/BP_lib/BPF_rev_OSCData_lib.Split floats To Vectors` _values (-1.0 1.0 1.0) (`self.Scale IN`)))
  (set `self.landmarksRow` _vecout)
  (`KismetSystemLibrary.Delay` 0.01)
  (`|ExecutionSequence`
    (:`then_0`
      (`/GenartLib/MediapipeFaceTracking/DynMesh.CreateFace` (`self.mesh`)))))

(event `self.Message Recived`
  (params (Message :type "OSCMessage Structure (by ref)") (IPAddress :type String) (Port :type Integer)))

(fn `UserConstructionScript`
  (`parent.UserConstructionScript`))